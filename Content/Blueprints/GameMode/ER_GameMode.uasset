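; Game mode for a timed, staged password puzzle session that starts on player restart and ends on a game-over widget.
; A self-rearming one-second timer counts down the current stage's time; NextSession rolls new passwords and switches to Stage 1.
; Passwords are a random four-digit code and a sequence code built from unique digits 0–3.
; Timeout sets the Succcessful stage and a correct password sets Lost, apparently inverted, with changes broadcast through dispatchers.
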(event Custom|NextSession
  (Password|InitPassword)
  (Stage|SetStage "NewEnumerator1")
  (CallFunction|StartSession))

(event Custom|StartSession
  (bind (_er_controller _result) (CallFunction|GetERPlayerController))
  ;[1 1 1] Inform the controller about the start of the session
  (if _result
    (Default|StartTimeSession _er_controller)
    ;[1 1 1] Start the countdown
    (Utilities|Time|SetTimerbyFunctionName self "TimeCalculate" 1.0)
    (Default|CallOnStartTimeSession)
    (EventDispatchers|BindEventtoOnTimeEnded (EventDispatchers|CreateEvent :!event Custom|OnTimeEnded_Event))
    (else
      (Development|PrintString "Error: no controller" true true "(R=1.000000,G=0.000000,B=0.000000,A=1.000000)"))))

(event Custom|TaskSuccess
  (Stage|SetStage "NewEnumerator2")
  (Default|ToggleWidget (.ER%20Controller (CallFunction|GetERPlayerController)) "/Game/Blueprints/Widgets/W_GameOver.W_GameOver_C"))

(event Custom|OnTimeEnded_Event
  (Stage|SetStage "NewEnumerator3")
  (Default|ToggleWidget (.ER%20Controller (CallFunction|GetERPlayerController)) "/Game/Blueprints/Widgets/W_GameOver.W_GameOver_C"))

(event EventBeginPlay
  (Audio|PushSoundMixModifier "/Game/Audio/AudioSettings/S_Volume_Mix.S_Volume_Mix"))

(event EventOnRestartPlayer
  (params (NewPlayer :type Controller%20Object%20Reference))
  (CallFunction|StartSession))

(fn ConstructionScript)

(fn GetRandomSequencePasword
  (Utilities|FlowControl|Sequence
    (:then_0
      ;[1 1 1] Creating unique numbers
      (LocalVariables|SetNewLocalVar_0 (Math|Random|RandomIntegerinRange 0 3)))
    (:then_1
      (LocalVariables|SetNewLocalVar_1 (Math|Random|RandomIntegerinRange 0 3))
      (Utilities|FlowControl|ForLoopwithBreak 0 1 :!label _label
        (:LoopBody
          (if (!= (LocalVariables|GetNewLocalVar_1) (LocalVariables|GetNewLocalVar_0))
            (goto _label Break)
            (else
              (bind _result (Math|Integer|IncrementInt (LocalVariables|GetNewLocalVar_1))
                (:%20%20
                  (if (> _result 3)
                    (LocalVariables|SetNewLocalVar_1 0)))))))))
    (:then_2
      (LocalVariables|SetNewLocalVar_2 (Math|Random|RandomIntegerinRange 0 3))
      (Utilities|FlowControl|ForLoopwithBreak 0 2 :!label _label_2
        (:LoopBody
          (if (and (!= (LocalVariables|GetNewLocalVar_2) (LocalVariables|GetNewLocalVar_0)) (!= (LocalVariables|GetNewLocalVar_2) (LocalVariables|GetNewLocalVar_1)))
            (goto _label_2 Break)
            (else
              (bind _result_2 (Math|Integer|IncrementInt (LocalVariables|GetNewLocalVar_2))
                (:%20%20
                  (if (> _result_2 3)
                    (LocalVariables|SetNewLocalVar_2 0)))))))))
    (:then_3
      (LocalVariables|SetNewLocalVar_3 (Math|Random|RandomIntegerinRange 0 3))
      (Utilities|FlowControl|ForLoopwithBreak 0 3 :!label _label_3
        (:LoopBody
          (if (Math|Boolean|ANDBoolean (!= (LocalVariables|GetNewLocalVar_3) (LocalVariables|GetNewLocalVar_0)) (!= (LocalVariables|GetNewLocalVar_3) (LocalVariables|GetNewLocalVar_1)) (!= (LocalVariables|GetNewLocalVar_3) (LocalVariables|GetNewLocalVar_2)))
            (goto _label_3 Break)
            (else
              (bind _result_3 (Math|Integer|IncrementInt (LocalVariables|GetNewLocalVar_3))
                (:%20%20
                  (if (> _result_3 3)
                    (LocalVariables|SetNewLocalVar_3 0)))))))))
    (:then_4
      (return (+ (* (LocalVariables|GetNewLocalVar_0) 1000) (* (LocalVariables|GetNewLocalVar_1) 100) (* (LocalVariables|GetNewLocalVar_2) 10) (LocalVariables|GetNewLocalVar_3))))))

(fn GetRandomPasword
  (return (Math|Random|RandomIntegerinRange 1000 9999)))

(fn TimeCalculate
  (if (> (Time|GetTimerSession) 0)
    (Utilities|FlowControl|Sequence
      (:then_0
        (switch Utilities|FlowControl|Switch|SwitchonE_StageSession (Variables|Stage|GetStage)
          (:NewEnumerator0
            (Math|Integer|DecrementInt (Variables|Time|GetTimeSessionStage_0)))
          (:NewEnumerator1
            (Math|Integer|DecrementInt (Variables|Time|GetTimeSessionStage_1)))))
      (:then_1
        (Utilities|Time|SetTimerbyFunctionName self "TimeCalculate" 1.0)))
    (else
      (Default|CallOnTimeEnded))))

(fn GetTimerSession
  (return (Utilities|Select :Index (Variables|Stage|GetStage) :NewEnumerator0 (Variables|Time|GetTimeSessionStage_0) :NewEnumerator1 (Variables|Time|GetTimeSessionStage_1) :NewEnumerator2 99 :NewEnumerator3 99)))

(fn AcceptPassword
  (params (Password :type Integer))
  (if (== Password (Variables|Password|GetPassword))
    (CallFunction|TaskSuccess)
    (return true)
    (else
      (return false))))

(fn InitPassword
  (Variables|Password|SetSequencePassword (Random|GetRandomSequencePasword))
  (Variables|Password|SetPassword (Random|GetRandomPasword)))

(fn GetSequencePassword
  (return (Variables|Password|GetSequencePassword)))

(fn GetPassword
  (return (Variables|Password|GetPassword)))

(fn SetStage
  (params (Stage :type E_StageSession%20Enum :default "NewEnumerator0"))
  (bind _output_get (Variables|Stage|SetStage Stage))
  (Default|CallOnChangedStageSession _output_get))

(fn GetStage
  (return (Variables|Stage|GetStage)))