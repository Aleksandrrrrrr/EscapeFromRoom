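; Game instance that applies and persists music and effects volume settings.
; SetAudioSettings overrides the music and effect sound classes in a shared sound mix, then saves to the SaveSettings slot; a negative value keeps that channel's stored volume.
; GetAudioSettings loads that slot, creating a default save if none exists.
; UpdateSettings pushes the mix and reapplies saved volumes; Init only sets a flag.
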(event EventInit
  (if (not (Variables|Default|GetbInit))
    (Variables|Default|SetbInit true)))

(fn SetAudioSettings
  (params (MusicVolume :type Float%20%28single-precision%29) (EffectVolume :type Float%20%28single-precision%29))
  (Utilities|FlowControl|Sequence
    (:then_0
      (if (>= MusicVolume 0.0)
        (Audio|SetSoundMixClassOverride "/Game/Audio/AudioSettings/S_Volume_Mix.S_Volume_Mix" "/Game/Audio/AudioSettings/S_Music_Class.S_Music_Class" MusicVolume 1.0 0.0 true)))
    (:then_1
      (if (>= EffectVolume 0.0)
        (Audio|SetSoundMixClassOverride "/Game/Audio/AudioSettings/S_Volume_Mix.S_Volume_Mix" "/Game/Audio/AudioSettings/S_Effect_Class.S_Effect_Class" EffectVolume 1.0 0.0 true)))
    (:then_2
      ;[1 1 1] Save settings
      (bind _returnvalue (SaveGame|CreateSaveGameObject "/Game/Blueprints/Save/SaveSettings.SaveSettings_C"))
      (Variables|/Game/Blueprints/Save/SaveSettings.SaveSettings_C|SetMusicVolume _returnvalue (select (>= MusicVolume 0.0) MusicVolume (.MusicVolume (CallFunction|GetAudioSettings))))
      (Variables|/Game/Blueprints/Save/SaveSettings.SaveSettings_C|SetEffectsVolume _returnvalue (select (>= EffectVolume 0.0) EffectVolume (.EffectVolume (CallFunction|GetAudioSettings))))
      (SaveGame|SaveGametoSlot _returnvalue "SaveSettings"))))

(fn GetAudioSettings
  (bind _returnvalue (SaveGame|DoesSaveGameExist "SaveSettings"))
  (if _returnvalue
    (bind _returnvalue_2 (SaveGame|LoadGamefromSlot "SaveSettings"))
    (bind _assave_settings (Utilities|Casting|CastToSaveSettings _returnvalue_2))
    (return (Variables|/Game/Blueprints/Save/SaveSettings.SaveSettings_C|GetMusicVolume _assave_settings) (Variables|/Game/Blueprints/Save/SaveSettings.SaveSettings_C|GetEffectsVolume _assave_settings))
    (else
      (bind _returnvalue_3 (SaveGame|CreateSaveGameObject "/Game/Blueprints/Save/SaveSettings.SaveSettings_C"))
      (SaveGame|SaveGametoSlot _returnvalue_3 "SaveSettings")
      (return (Variables|/Game/Blueprints/Save/SaveSettings.SaveSettings_C|GetMusicVolume _returnvalue_3) (Variables|/Game/Blueprints/Save/SaveSettings.SaveSettings_C|GetEffectsVolume _returnvalue_3)))))

(fn UpdateSettings
  (bind (_musicvolume _effectvolume) (CallFunction|GetAudioSettings))
  (Audio|PushSoundMixModifier "/Game/Audio/AudioSettings/S_Volume_Mix.S_Volume_Mix")
  (CallFunction|SetAudioSettings _musicvolume _effectvolume))