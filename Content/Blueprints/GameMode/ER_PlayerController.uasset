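; ER player controller that manages on-screen widgets and input modes across a timed session.
; On BeginPlay it binds to the ER game mode's session-start and time-ended delegates, showing HUD and info widgets at start and a game over widget at timeout.
; Helper functions clear widgets and switch between UI-only and game-only input.
; Restart and quit events run console commands.
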(event Custom|TimeEnded
  ;[1 1 1] Call game over widget
  (CallFunction|ToggleWidget "/Game/Blueprints/Widgets/W_GameOver.W_GameOver_C"))

(event Custom|StartTimeSession
  ;[1 1 1] Create HUD widget
  (bind _returnvalue (UserInterface|CreateWidget "/Game/Blueprints/Widgets/W_HUD.W_HUD_C" self))
  (UserInterface|Viewport|AddtoViewport _returnvalue 0)
  (Input|SetInputModeGameOnly self)
  ;[1 1 1] Call inform widget
  (bind _returnvalue_2 (UserInterface|CreateWidget "/Game/Blueprints/Widgets/W_Info.W_Info_C" self))
  (UserInterface|Viewport|AddtoViewport _returnvalue_2 0))

(event Custom|RestartSession
  (Development|ExecuteConsoleCommand "RestartLevel" 0))

(event Custom|QuitGame
  (Development|ExecuteConsoleCommand "Exit" 0))

(event EventBeginPlay
  (CallFunction|Init))

(fn ConstructionScript)

(fn ToggleWidget
  (params (WidgetClass :type User%20Widget%20Class%20Reference))
  (Viewport|RemoveAllWidgets)
  (bind _returnvalue (UserInterface|CreateWidget WidgetClass self))
  (UserInterface|Viewport|AddtoViewport _returnvalue 0)
  (Input|SetInputModeUIOnly self _returnvalue "DoNotLock"))

(fn FocusinGame
  (Viewport|RemoveAllWidgets)
  (bind _returnvalue (UserInterface|CreateWidget "/Game/Blueprints/Widgets/W_HUD.W_HUD_C" self))
  (UserInterface|Viewport|AddtoViewport _returnvalue 0)
  (Input|SetInputModeGameOnly self))

(fn Init
  (bind (_er_game_mode _result) (CallFunction|GetERGameMode))
  (if _result
    (EventDispatchers|BindEventtoOnTimeEnded _er_game_mode (EventDispatchers|CreateEvent :!event Custom|TimeEnded))
    (EventDispatchers|BindEventtoOnStartTimeSession _er_game_mode (EventDispatchers|CreateEvent :!event Custom|StartTimeSession))))