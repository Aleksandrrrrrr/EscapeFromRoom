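; StorageComponent is a component that stores a list of items, looked up by name, with functions to query, add, remove and use them.
; AddItem always appends and succeeds, while RemoveItem first checks that the name is present.
; UseItem consumes an item by removing it through RemoveItem.
; Each successful change fires an event dispatcher for added, removed or used items, so using an item signals both removal and use.
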(event EventBeginPlay)

(event EventTick
  (params (DeltaSeconds :type Float%20%28single-precision%29)))

(fn GetItems
  (return (Variables|Default|GetItems)))

(fn CheckItembyName
  (params (Name :type Name))
  (for _array_element (Data|GetItems)
    (if (Utilities|Name|Equal(Name) Name _array_element)
      (return true)))
  (return false))

(fn AddItem
  (params (NewItem :type Name%20%28by%20ref%29))
  (Utilities|Array|Add (Variables|Default|GetItems) NewItem)
  (Default|CallOnItemAdded NewItem)
  (return true))

(fn RemoveItem
  (params (NameItem :type Name))
  (if (Data|CheckItembyName NameItem)
    (bind _returnvalue (Utilities|Array|RemoveItem (Variables|Default|GetItems) NameItem))
    (if _returnvalue
      (Default|CallOnRemoveItem NameItem)
      (return true)
      (else
        _)))
  (return false))

(fn UseItem
  (params (NameItem :type Name))
  (if (Data|CheckItembyName NameItem)
    (bind _result (CallFunction|RemoveItem NameItem))
    (if _result
      (Default|CallOnItemUsed NameItem)
      (return true)
      (else
        _)))
  (return false))