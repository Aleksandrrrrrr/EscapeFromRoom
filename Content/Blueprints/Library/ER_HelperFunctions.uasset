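; ER_HelperFunctions is a Blueprint library of shared helpers for the ER game.
; Getters cast player 0's character and controller and the game mode, each with a success flag, plus the game instance without one.
; Other helpers format non-negative times as zero-padded minutes:seconds, extract one digit from a four-digit number, and turn an input action's first mapped key into quoted display text.
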(fn GetERCharacter
  (bind _aser_character (Utilities|Casting|CastToER_Character (Game|GetPlayerCharacter 0))
    (:then
      (return _aser_character true))
    (:CastFailed
      (return 0 false))))

(fn GetERPlayerController
  (bind _aser_player_controller (Utilities|Casting|CastToER_PlayerController (Game|GetPlayerController 0))
    (:then
      (return _aser_player_controller true))
    (:CastFailed
      (return 0 false))))

(fn GetERGameMode
  (bind _aser_game_mode (Utilities|Casting|CastToER_GameMode (Game|GetGameMode))
    (:then
      (return _aser_game_mode true))
    (:CastFailed
      (return 0 false))))

(fn DatetoString
  (params (InTime :type Integer))
  (if (>= InTime 0)
    (return (|TimeCalculated_2))
    (else
      (return ""))))

(fn DateStringPrefix
  (params (A :type Integer))
  (return (select (< A 10) "0" "")))

(fn GetKeytoText
  (params (InActionName :type Name))
  (return (Utilities|Text|ToText(String) (Utilities|String|Append "\"" (Utilities|String|ToString(Text) (Class|KismetInputLibrary|KeyGetDisplayName (Key|GetKeybyName InActionName))) "\""))))

(fn GetKeybyName
  (params (InActionName :type Name))
  (return (Utilities|Struct|BreakInputActionKeyMapping (Utilities|Array|Get(acopy) (Class|InputSettings|GetActionMappingbyName (Class|InputSettings|GetInputSettings) InActionName)))))

(fn GetNumberbyIndex
  (params (Index :type Integer) (Number :type Integer))
  (return (Utilities|Select :Index Index :Option%200 (/ Number 1000) :Option%201 (/ (Math|Integer|%(Integer) Number 1000) 100) :Option%202 (/ (Math|Integer|%(Integer) Number 100) 10) :Option%203 (Math|Integer|%(Integer) Number 10))))

(fn GetERGameInstance
  (return (.AsER%20Game%20Instance (Utilities|Casting|CastToER_GameInstance (Game|GetGameInstance)))))