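; DisplayNumber is an actor that reveals one digit of the game mode's password on a text render component.
; It listens for the ER game mode's stage session change and reacts to one specific stage.
; It searches four positions of the sequence password for its own Number, then shows the password digit at the matching position, so the sequence determines which digit each display shows.
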(event Custom|OnChangedStageSession
  (params (Stage :type E_StageSession%20Enum :default "NewEnumerator0"))
  (if (Utilities|Enum|Equal(Enum) Stage "NewEnumerator1")
    (bind _index (Utilities|FlowControl|ForLoopwithBreak 0 3 :!label _label)
      (:LoopBody
        (Utilities|SearchforSelfNumber _index
          (:true
            (Rendering|Components|TextRender|SetText (Variables|Default|GetTextRender) (Utilities|Text|ToText(Integer) (CallFunction|GetNumberbyIndex _index (Default|GetPassword (.ER%20Game%20Mode (CallFunction|GetERGameMode))))))
            (goto _label Break)))))))

(event EventBeginPlay
  (bind (_er_game_mode _result) (CallFunction|GetERGameMode))
  (if _result
    (EventDispatchers|AssignOnChangedStageSession _er_game_mode (EventDispatchers|CreateEvent :!event Custom|OnChangedStageSession))))

(fn ConstructionScript)