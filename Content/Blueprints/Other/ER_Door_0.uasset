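; Key-locked door actor that swings open once an interacting instigator carries the key.
; Interact looks up "I_Key" in the instigator's StorageManager, sets a Used flag on success and returns the result, without removing the key.
; Tick calls OpenDoor, which, while Used is set, eases the Cube's world yaw toward a fixed absolute angle with FInterpTo.
; Nothing resets the flag or closes the door.
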(event EventBeginPlay)

(event Collision|EventActorBeginOverlap
  (params (OtherActor :type Actor%20Object%20Reference)))

(event EventTick
  (params (DeltaSeconds :type Float%20%28single-precision%29))
  (Utilities|OpenDoor))

(fn ConstructionScript)

(fn Interact
  (params (Instigator :type ER%20Character%20Object%20Reference))
  (if (Default|CheckItembyName (Variables|/Game/Blueprints/GameMode/ER_Character.ER_Character_C|GetStorageManager Instigator) "I_Key")
    (Variables|Default|SetUsed true)
    (return true)
    (else
      (return false))))