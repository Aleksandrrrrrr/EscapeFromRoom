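; Guard actor that displays one element of the session password on a W_Guard widget.
; On BeginPlay it binds to the ER game mode's stage-session change event, printing an error if that game mode is missing.
; When a specific stage begins, it picks the digit at its Number index from the game mode's password sequence.
; It passes that digit as the guard type to its widget component.
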(event Custom|SetGuardType
  (params (Type :type Integer))
  (bind _asw_guard (Utilities|Casting|CastToW_Guard (UserInterface|GetUserWidgetObject (Variables|Default|GetWidget))))
  (Default|SetType _asw_guard Type))

(event Custom|OnChangedStageSession
  (params (Stage :type E_StageSession%20Enum :default "NewEnumerator0"))
  (if (Utilities|Enum|Equal(Enum) Stage "NewEnumerator1")
    (CallFunction|SetGuardType (CallFunction|GetNumberbyIndex (Variables|Default|GetNumber) (Default|GetSequencePassword (.ER%20Game%20Mode (CallFunction|GetERGameMode)))))))

(event EventBeginPlay
  (bind (_er_game_mode _result) (CallFunction|GetERGameMode))
  (if _result
    (EventDispatchers|AssignOnChangedStageSession _er_game_mode (EventDispatchers|CreateEvent :!event Custom|OnChangedStageSession))
    (else
      (Development|PrintString "Error: not game mode" true true "(R=1.000000,G=0.000000,B=0.000000,A=1.000000)"))))

(fn ConstructionScript)